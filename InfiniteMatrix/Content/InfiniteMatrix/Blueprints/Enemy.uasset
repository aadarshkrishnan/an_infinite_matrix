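; Enemy actor that damages the player on contact and is destroyed by projectiles, using events on its Sphere component.
; A sphere hit on BP_Player subtracts health, destroys the enemy, and flags death and shows the restart display once health runs out.
; A Projectile overlap destroys both actors, then casts that same overlapping actor to BP_Player to add score, so scoring requires it to be both types.
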(event `self.Sphere.OnComponentHit`
  (params (HitComponent :type "PrimitiveComponent Object Reference") (OtherActor :type "Actor Object Reference") (OtherComp :type "PrimitiveComponent Object Reference") (NormalImpulse :type "Vector Structure") (Hit :type "HitResult Structure (by ref)"))
  (bind _asbp_player (cast `/Game/InfiniteMatrix/Blueprints/BP_Player` OtherActor))
  (set `/Game/InfiniteMatrix/Blueprints/BP_Player.Health` (- (`/Game/InfiniteMatrix/Blueprints/BP_Player.Health` _asbp_player) 20.0) _asbp_player)
  (`self.K2_DestroyActor` self)
  (if (<= (`/Game/InfiniteMatrix/Blueprints/BP_Player.Health` _asbp_player) 0.0)
    (set `/Game/InfiniteMatrix/Blueprints/BP_Player.isDead` true _asbp_player)
    (`/Game/InfiniteMatrix/Blueprints/BP_Player.Display Restart` _asbp_player)))

(event `self.Sphere.OnComponentBeginOverlap`
  (params (OverlappedComponent :type "PrimitiveComponent Object Reference") (OtherActor :type "Actor Object Reference") (OtherComp :type "PrimitiveComponent Object Reference") (OtherBodyIndex :type Integer) (bFromSweep :type Boolean) (SweepResult :type "HitResult Structure (by ref)"))
  (bind _asprojectile (cast `/Game/InfiniteMatrix/Blueprints/Projectile` OtherActor))
  (`self.K2_DestroyActor` _asprojectile)
  (`self.K2_DestroyActor`)
  (bind _asbp_player (cast `/Game/InfiniteMatrix/Blueprints/BP_Player` OtherActor))
  (set `/Game/InfiniteMatrix/Blueprints/BP_Player.Score` (+ (`/Game/InfiniteMatrix/Blueprints/BP_Player.Score` _asbp_player) 1.0) _asbp_player))

(fn `UserConstructionScript`)